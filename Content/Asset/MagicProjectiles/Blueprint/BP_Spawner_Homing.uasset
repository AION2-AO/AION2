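; Projectile spawner actor that repeatedly fires a configurable projectile class with a muzzle flash effect.
; After a start delay, BeginPlay fires once and starts a looping timer at the FireRate interval.
; A Timeline played from Tick rotates the root, changing the direction projectiles spawn in.
; Spawns sit at a fixed world X offset, and the flash uses the Arrow's relative rotation rather than the actor's.
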(event `self.ReceiveTick`
  (params (DeltaSeconds :type "Float (single-precision)"))
  ; Rotation
  (bind (_direction _rotation_1 _roation_2) (`Timeline|Timeline`)
    (:`Update`
      (bind _returnvalue (* _rotation_1 75.0))
      (`SceneComponent.K2_SetRelativeRotation` (`self.DefaultSceneRoot`) (`KismetMathLibrary.MakeRotator` _returnvalue (* _roation_2 75.0) _returnvalue) false false))))

(event `self.ReceiveBeginPlay`
  (`KismetSystemLibrary.Delay` (`self.StartDelay`))
  (`self.SpawnFX`)
  (`KismetSystemLibrary.K2_SetTimerDelegate` (delegate `SpawnFX`) (`self.FireRate`) true))

(event `SpawnFX`
  (`NiagaraFunctionLibrary.SpawnSystemAtLocation` (`self.MuzzleFlashFX`) (+ (`self.K2_GetActorLocation`) (40.0 0.0 0.0)) (`SceneComponent.RelativeRotation` (`self.Arrow`)))
  (`|SpawnActorFromClass` (`self.ProjectileClass`) (`KismetMathLibrary.MakeTransform` (+ (`self.K2_GetActorLocation`) (40.0 0.0 0.0)) (`self.K2_GetActorRotation`)) "Undefined" "MultiplyWithRoot" null (`self.GetInstigator`)))

(fn `UserConstructionScript`)