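; BP_Projectile is a homing magic projectile with configurable Niagara projectile and impact effects.
; On BeginPlay it sets the projectile effect and locks ProjectileMovement onto the nearest "Homing"-tagged actor under the ClosestDistance threshold, using that actor's scene component.
; The first sphere overlap spawns the impact effect aligned to the sweep normal, deactivates the projectile effect and destroys the actor after a short delay.
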(event `self.ReceiveBeginPlay`
  (`self.Lock On`)
  (`NiagaraComponent.SetAsset` (`self.Projectile`) (`self.ProjectileFX`) true))

(event `self.Sphere.OnComponentBeginOverlap`
  (params (OverlappedComponent :type "PrimitiveComponent Object Reference") (OtherActor :type "Actor Object Reference") (OtherComp :type "PrimitiveComponent Object Reference") (OtherBodyIndex :type Integer) (bFromSweep :type Boolean) (SweepResult :type "HitResult Structure (by ref)"))
  (if (not (`self.HasCollided`))
    (`NiagaraFunctionLibrary.SpawnSystemAtLocation` (`self.ImpactFX`) (`self.K2_GetActorLocation`) (`KismetMathLibrary.MakeRotFromX` (`.ImpactNormal` (`GameplayStatics.BreakHitResult` SweepResult))))
    (`ActorComponent.Deactivate` (`self.Projectile`))
    (set `self.HasCollided` true)
    (`KismetSystemLibrary.Delay` 2.0)
    (`self.K2_DestroyActor`)))

(event `Lock On`
  (bind _projectilemovement (`self.ProjectileMovement`))
  ; Homing
  (bind _homing_target (`self.Find Homing Target`))
  (set `ProjectileMovementComponent.HomingTargetComponent` _homing_target _projectilemovement)
  (set `ProjectileMovementComponent.bIsHomingProjectile` true _projectilemovement))

(fn `Find Homing Target`
  (returns (`Homing Target` :type "SceneComponent Object Reference"))
  (bind _outactors (`GameplayStatics.GetAllActorsOfClassWithTag` "/Script/Engine.Actor" "Homing"))
  (for _array_element _outactors
    (bind _returnvalue (`KismetMathLibrary.VSize` (- (`self.K2_GetActorLocation` _array_element) (`self.K2_GetActorLocation`))))
    (if (< _returnvalue (`self.Closest Distance`))
      (set `self.Closest Distance` _returnvalue)
      (set `self.Homing Target` _array_element)))
  (return (`self.GetComponentByClass` (`self.Homing Target`) "/Script/Engine.SceneComponent")))

(fn `UserConstructionScript`)