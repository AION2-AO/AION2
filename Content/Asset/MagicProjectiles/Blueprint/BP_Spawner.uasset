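; BP_Spawner is an actor that repeatedly fires magic projectiles on a timer.
; After a start delay on BeginPlay, it fires once and starts a looping timer at the FireRate interval.
; Each shot spawns a muzzle flash system at the actor location using the Arrow's relative rotation, then spawns ProjectileClass at the actor's transform, passing on its Instigator.
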(event `self.ReceiveBeginPlay`
  (`KismetSystemLibrary.Delay` (`self.StartDelay`))
  (`self.SpawnFX`)
  (`KismetSystemLibrary.K2_SetTimerDelegate` (delegate `SpawnFX`) (`self.FireRate`) true))

(event `SpawnFX`
  (`NiagaraFunctionLibrary.SpawnSystemAtLocation` (`self.MuzzleFlashFX`) (`self.K2_GetActorLocation`) (`SceneComponent.RelativeRotation` (`self.Arrow`)))
  (`|SpawnActorFromClass` (`self.ProjectileClass`) (`self.GetTransform`) "Undefined" "MultiplyWithRoot" null (`self.GetInstigator`)))

(fn `UserConstructionScript`)